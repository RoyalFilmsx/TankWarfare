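; Player-controlled tank pawn with driving, camera look, right-mouse zoom and an overhead name tag.
; Axis inputs offset and rotate the main body with teleport and feed controller pitch and yaw, while a timeline drives camera FOV for zoom.
; Authority copies the PS_Tank player name after a short delay, and RepNotify or a remote update event writes it to the W_TankID widget.
; Key 1 subtracts random, clamped health.
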(event Custom|S_SetPlayerNames
  ;[1 1 1] PlayerNames
  (Utilities|FlowControl|Delay 0.5)
  (bind _asps_tank (Utilities|Casting|CastToPS_Tank (Variables|GetPlayerState)))
  (Variables|Default|SetSetPlayerName (Variables|/Script/Engine.PlayerState|GetPlayerName _asps_tank)))

(event Custom|C_UpdatePlayerName
  ;[1 1 1] PlayerNames
  (bind _asw_tank_id (Utilities|Casting|CastToW_TankID (UserInterface|GetUserWidgetObject (Variables|Default|GetW_PlayerTag))))
  (Rendering|Components|TextRender|SetText (Variables|/Game/TankWarfareCore/Widgets/W_TankID.W_TankID_C|GetPlayerName _asw_tank_id) (Utilities|Text|ToText(String) (Variables|Default|GetSetPlayerName))))

(event EventBeginPlay
  ;[1 1 1] PlayerNames
  (Networking|SwitchHasAuthority
    (:Authority
      (CallFunction|SSetPlayerNames))
    (:Remote
      (CallFunction|CUpdatePlayerName))))

(event Input|AxisEvents|InputAxisMoveForward
  (params (AxisValue :type Float%20%28single-precision%29))
  (Transformation|AddLocalOffset (Variables|Default|GetTank_MainBody) (Math|Vector|MakeVector (* AxisValue (Variables|Default|GetTank_Speed)) 0.0 0.0) false true))

(event Input|AxisEvents|InputAxisTurnRight
  (params (AxisValue :type Float%20%28single-precision%29))
  (Transformation|AddWorldRotation (Variables|Default|GetTank_MainBody) (Math|Rotator|MakeRotator 0.0 0.0 AxisValue) false true))

(event Input|AxisEvents|InputAxisLookUp
  (params (AxisValue :type Float%20%28single-precision%29))
  (Pawn|Input|AddControllerPitchInput AxisValue))

(event Input|AxisEvents|InputAxisLookRight
  (params (AxisValue :type Float%20%28single-precision%29))
  (Pawn|Input|AddControllerYawInput AxisValue))

(event Input|KeyboardEvents|SpaceBar
  (params (Key :type Key%20Structure :default "None")))

(event Input|KeyboardEvents|1
  (params (Key :type Key%20Structure :default "None"))
  (:Pressed
    (Variables|Default|SetDamageNumberFloat 0.25)
    (Variables|Default|SetCurrentHealth (Math|Float|Clamp(Float) (- (Variables|Default|GetCurrentHealth) (Math|Random|RandomFloatinRange 0.1 0.3))))))

(event Input|MouseEvents|RightMouseButton
  (params (Key :type Key%20Structure :default "None"))
  ;[1 1 1] Zoom
  (:Pressed
    (Variables|Default|SetisInZoom? true)
    (bind _newtrack_0 (Timeline|Timeline_0 PlayFromStart)
      (:Update
        (Camera|SetFieldOfView (Variables|Default|GetCamera) _newtrack_0))))
  (:Released
    (Variables|Default|SetisInZoom? false)
    (Timeline|Timeline_0 ReverseFromEnd)))

(fn ConstructionScript)

(fn OnRepSetPlayerName
  (bind _asw_tank_id (Utilities|Casting|CastToW_TankID (UserInterface|GetUserWidgetObject (Variables|Default|GetW_PlayerTag))))
  (Rendering|Components|TextRender|SetText (Variables|/Game/TankWarfareCore/Widgets/W_TankID.W_TankID_C|GetPlayerName _asw_tank_id) (Utilities|Text|ToText(String) (Variables|Default|GetSetPlayerName))))