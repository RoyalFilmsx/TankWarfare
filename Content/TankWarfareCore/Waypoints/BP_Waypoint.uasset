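; BP_Waypoint is a chained objective marker in the tank game that hands off to the next waypoint when reached.
; When a BP_Tank overlaps its sphere while active, it activates NextWayPoint and deactivates itself.
; The active flag controls the widget component's visibility.
; While active, Tick writes the player character's halved, truncated distance to the W_Waypoint widget as a label in meters.
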(event OnComponentBeginOverlap(Sphere)
  (params (OverlappedComponent :type Primitive%20Component%20Object%20Reference) (OtherActor :type Actor%20Object%20Reference) (OtherComp :type Primitive%20Component%20Object%20Reference) (OtherBodyIndex :type Integer) (bFromSweep :type Boolean) (SweepResult :type Hit%20Result%20Structure%20%28by%20ref%29))
  (Utilities|Casting|CastToBP_Tank OtherActor)
  (if (Variables|Waypoints|GetActive?)
    (CallFunction|ActivateWayPoint (Variables|Waypoints|GetNextWayPoint))
    (CallFunction|DeactivateWaypoint)))

(event Custom|ActivateWayPoint
  (bind _output_get (Variables|Waypoints|SetActive? true))
  (Rendering|SetVisibility (Variables|Default|GetWidget) _output_get false))

(event Custom|DeactivateWaypoint
  (bind _output_get (Variables|Waypoints|SetActive? false))
  (Rendering|SetVisibility (Variables|Default|GetWidget) _output_get false))

(event EventBeginPlay
  (Rendering|SetVisibility (Variables|Default|GetWidget) (Variables|Waypoints|GetActive?) false)
  (bind _asw_waypoint (Utilities|Casting|CastToW_Waypoint (UserInterface|GetUserWidgetObject (Variables|Default|GetWidget))))
  (Variables|Default|SetWidget_REF _asw_waypoint))

(event EventTick
  (params (DeltaSeconds :type Float%20%28single-precision%29))
  (if (Variables|Waypoints|GetActive?)
    (Variables|/Game/TankWarfareCore/Waypoints/W_Waypoint.W_Waypoint_C|SetDistanceText (Variables|Default|GetWidget_REF) (Utilities|String|Append (Utilities|String|ToString(Integer) (/ (Math|Float|Truncate (Math|Vector|Distance(Vector) (Transformation|GetActorLocation (Game|GetPlayerCharacter 0)) (Transformation|GetActorLocation))) 2)) "m"))))

(fn ConstructionScript)